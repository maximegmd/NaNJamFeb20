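; FutureSword is a melee weapon that damages other GJCharacters it overlaps while its wielder is alive and attacking.
; Hits are server-only and skip characters of the wielder's exact class, so same-class allies are unharmed.
; A map of each victim to the wielder's attack count limits damage to once per swing.
; Each hit triggers WeaponHit for particles and a random slash sound, then adds score if the wielder is a PlayerCharacter.
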(event `self.ReceiveActorBeginOverlap`
  (params (OtherActor :type "Actor Object Reference"))
  (bind _returnvalue (`self.GetCharacter`))
  (bind _othercharacter (`self.OtherCharacter`))
  (bind _attackactioncount (`GJCharacter.AttackActionCount` _returnvalue))
  (`/Engine/EditorBlueprintResources/StandardMacros.IsValid` _returnvalue
    (:`Is Valid`
      (if (and (`GJCharacter.bPerformingAttack` _returnvalue) (> (`GJCharacter.Health` _returnvalue) 0.0001))
        (bind _asgjcharacter (cast `GJCharacter` OtherActor))
        (set `self.OtherCharacter` _asgjcharacter)
        (if (== _asgjcharacter _returnvalue)
          _
          (elif (and (`KismetSystemLibrary.IsServer`) (!= (`GameplayStatics.GetObjectClass` _returnvalue) (`GameplayStatics.GetObjectClass` (`self.OtherCharacter`))))
            (if (!= _attackactioncount (`BlueprintMapLibrary.Map_Find` (`self.LastHitCount`) (`self.OtherCharacter`)))
              (`BlueprintMapLibrary.Map_Add` (`self.LastHitCount`) (`self.OtherCharacter`) _attackactioncount)
              (`GameplayStatics.ApplyDamage` _othercharacter 10.0 null (`self.GetCharacter`))
              (bind _assound_wave (cast `SoundWave` (`KismetMathLibrary.SelectObject` "/Game/GameJam/Sound/Sword_Slash_1_v1.Sword_Slash_1_v1" "/Game/GameJam/Sound/Sword_Slash_1_v2.Sword_Slash_1_v2" (`KismetMathLibrary.RandomBool`))))
              (`self.WeaponHit` (+ (0.0 0.0 80.0) (`SceneComponent.K2_GetComponentLocation` (`Character.Mesh` _othercharacter))) _assound_wave)
              (bind _asplayer_character (cast `/Game/GameJam/Blueprints/PlayerCharacter` (`self.GetCharacter`)))
              (set `/Game/GameJam/Blueprints/PlayerCharacter.Score` (+ (`/Game/GameJam/Blueprints/PlayerCharacter.Score` _asplayer_character) 100) _asplayer_character))))))))

(event `WeaponHit`
  (params (Location :type "Vector Structure") (Sound :type "SoundWave Object Reference"))
  (`GameplayStatics.SpawnEmitterAtLocation` "/Game/FXVarietyPack/Particles/P_ky_hit1.P_ky_hit1" Location (struct) (0.5 0.5 0.5))
  (`GameplayStatics.PlaySoundAtLocation` Sound (0.0 0.0 0.0) (struct) 0.5 1.0 0.0 null null null))

(fn `UserConstructionScript`)