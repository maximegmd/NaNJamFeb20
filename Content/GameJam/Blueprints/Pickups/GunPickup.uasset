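; GunPickup is a pickup actor that gives a weapon to any GJCharacter that overlaps it.
; On overlap, if that character has authority, the pickup destroys itself and passes its WeaponClass to PickUpWeapon.
; For a PlayerCharacter, it also appends the class to WeaponInventory, sets Index to the new slot and prints that index.
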(event `self.ReceiveActorBeginOverlap`
  (params (OtherActor :type "Actor Object Reference"))
  (bind _weaponclass (`self.WeaponClass`))
  (bind _asgjcharacter (cast `GJCharacter` OtherActor))
  (if (`self.HasAuthority` _asgjcharacter)
    (`self.K2_DestroyActor` self)
    (`GJCharacter.PickUpWeapon` _asgjcharacter _weaponclass)
    (bind _asplayer_character (cast `/Game/GameJam/Blueprints/PlayerCharacter` _asgjcharacter))
    (bind _returnvalue (`KismetArrayLibrary.Array_Add` (`/Game/GameJam/Blueprints/PlayerCharacter.WeaponInventory` _asplayer_character) _weaponclass))
    (bind _output_get (set `/Game/GameJam/Blueprints/PlayerCharacter.index` _returnvalue _asplayer_character))
    (`KismetSystemLibrary.PrintString` (`KismetStringLibrary.Conv_IntToString` _output_get))))

(fn `UserConstructionScript`)