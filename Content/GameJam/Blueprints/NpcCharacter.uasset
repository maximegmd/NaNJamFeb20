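; NPC character Blueprint for an armed, melee-capable character that ragdolls on death.
; On the authority it picks a random skeletal mesh at construction and equips its weapon class through WeaponComponent at BeginPlay.
; Damage that would leave Health near zero triggers Die and blocks controller movement; this graph never writes Health back.
; Die enables mesh physics, disables capsule collision, then unequips and destroys the actor after a delay.
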(event `self.ReceiveBeginPlay`
  (`/Engine/EditorBlueprintResources/ActorMacros.Switch Has Authority`
    (:`Authority`
      (`GJWeaponComponent.Equip` (`self.WeaponComponent`) (`self.WeaponClass`)))))

(event `/Game/GameJam/Blueprints/CombatInterface.MeleeAttack`
  (`self.ImmediateSimpleAttack`))

(event `self.ReceiveAnyDamage`
  (params (Damage :type "Float (single-precision)") (DamageType :type "DamageType Object Reference") (InstigatedBy :type "Controller Object Reference") (DamageCauser :type "Actor Object Reference"))
  (if (<= (- (`self.Health`) Damage) 0.1)
    (`self.Die`)
    (`Controller.SetIgnoreMoveInput` (`self.GetController`) true)))

(event `Die`
  (bind _capsulecomponent (`self.CapsuleComponent`))
  (bind _mesh (`self.Mesh`))
  (`PrimitiveComponent.SetSimulatePhysics` _mesh true)
  (`PrimitiveComponent.SetCollisionEnabled` _mesh "PhysicsOnly")
  (`SkeletalMeshComponent.ResetAllBodiesSimulatePhysics` (`self.Mesh`))
  (set `PrimitiveComponent.bGenerateOverlapEvents` false _capsulecomponent)
  (`PrimitiveComponent.SetCollisionEnabled` _capsulecomponent "NoCollision")
  (`KismetSystemLibrary.Delay` 5.0)
  (`GJWeaponComponent.Unequip` (`self.WeaponComponent`))
  (`self.K2_DestroyActor`))

(fn `UserConstructionScript`
  (bind _meshrefs (`self.MeshRefs`))
  (`/Engine/EditorBlueprintResources/ActorMacros.Switch Has Authority`
    (:`Authority`
      (`SkinnedMeshComponent.SetSkinnedAssetAndUpdate` (`self.Mesh`) (`|GetArrayItem` _meshrefs (`KismetMathLibrary.RandomInteger` (`KismetArrayLibrary.Array_Length` _meshrefs))) false))))