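; Player character Blueprint that keeps a weapon inventory and cycles through it on input.
; BeginPlay adds WeaponClass to WeaponInventory and sets Index to the new entry, without equipping it.
; Pressing SelectNextWeapon has WeaponComponent unequip, then equip the entry at Index, and only afterwards advances Index with wraparound.
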(event `InputAction|SelectNextWeapon`
  (params (Key :type "Key Structure"))
  (:`Pressed`
    (`GJWeaponComponent.Unequip` (`self.WeaponComponent`))
    (`GJWeaponComponent.Equip` (`self.WeaponComponent`) (`|GetArrayItem` (`self.WeaponInventory`) (`self.index`)))
    (set `self.index` (mod (+ (`self.index`) 1) (`KismetArrayLibrary.Array_Length` (`self.WeaponInventory`))))))

(event `self.ReceiveBeginPlay`
  (bind _returnvalue (`KismetArrayLibrary.Array_Add` (`self.WeaponInventory`) (`self.WeaponClass`)))
  (set `self.index` _returnvalue))

(fn `UserConstructionScript`)