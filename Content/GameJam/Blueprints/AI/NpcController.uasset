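; AI controller for NPC characters that runs the NPC behavior tree and feeds it which player to chase.
; On possessing an NpcCharacter, the server caches the pawn and starts NPC_BT.
; Server-side perception updates maintain a list of sensed PlayerCharacters, then write the CanSeePlayer flag and the first listed player as ActorToChase to the blackboard, clearing the target when none remain.
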(event `self.ReceivePossess`
  (params (PossessedPawn :type "Pawn Object Reference"))
  ;[1 1 1] Enable AI
  (`/Engine/EditorBlueprintResources/ActorMacros.Switch Has Authority`
    (:`Authority`
      (bind _asnpc_character (cast `/Game/GameJam/Blueprints/NpcCharacter` PossessedPawn))
      (set `self.MyPawn` _asnpc_character)
      (`self.RunBehaviorTree` "/Game/GameJam/Blueprints/AI/NPC_BT.NPC_BT"))))

(event `self.AIPerception.OnTargetPerceptionUpdated`
  (params (Actor :type "Actor Object Reference") (Stimulus :type "AIStimulus Structure"))
  (bind _returnvalue (`AIBlueprintHelperLibrary.GetBlackboard` null))
  (bind _charactersinview (`self.CharactersInView`))
  (bind _returnvalue_2 (> (`KismetArrayLibrary.Array_Length` _charactersinview) 0))
  ;[1 1 1] Character Perception
  (`/Engine/EditorBlueprintResources/ActorMacros.Switch Has Authority`
    (:`Authority`
      (bind _asplayer_character (cast `/Game/GameJam/Blueprints/PlayerCharacter` Actor))
      (if (`.bSuccessfullySensed` (break `AIStimulus` Stimulus))
        (`KismetArrayLibrary.Array_Add` (`self.CharactersInView`) _asplayer_character)
        (else
          (`KismetArrayLibrary.Array_RemoveItem` (`self.CharactersInView`) _asplayer_character)))
      (`BlackboardComponent.SetValueAsBool` _returnvalue "CanSeePlayer" _returnvalue_2)
      (if _returnvalue_2
        (`BlackboardComponent.SetValueAsObject` _returnvalue "ActorToChase" (`|GetArrayItem` _charactersinview))
        (else
          (`BlackboardComponent.SetValueAsObject` _returnvalue "ActorToChase" null))))))

(fn `UserConstructionScript`)